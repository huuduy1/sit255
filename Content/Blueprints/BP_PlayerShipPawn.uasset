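; BP_PlayerShipPawn is the player's ship pawn, which adds the BP_playerHUD widget to the viewport on BeginPlay.
; Its Fire function spawns a BP_Projectile_CannonBall at a given cannon's transform, passing in damage, radius, impulse and velocity.
; Broadside calls for four right and four left cannons exist in the event graph, but no event triggers them.
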(event `self.ReceiveBeginPlay`
  (bind _returnvalue (`|CreateWidget` "/Game/Blueprints/BP_playerHUD.BP_playerHUD_C"))
  (`UserWidget.AddToViewport` _returnvalue 0))

(event `self.ReceiveTick`
  (params (DeltaSeconds :type "Float (single-precision)")))

(fn `Fire`
  (params (Cannon :type "ArrowComponent Object Reference"))
  (bind (_returnvalue_location _returnvalue_rotation _returnvalue_scale) (`KismetMathLibrary.BreakTransform` (`SceneComponent.K2_GetComponentToWorld` Cannon)))
  (`|SpawnActorFromClass` "/Game/Cannon/Cannonz/BP_Projectile_CannonBall.BP_Projectile_CannonBall_C" (`KismetMathLibrary.MakeTransform` _returnvalue_location _returnvalue_rotation _returnvalue_scale) "AlwaysSpawn" "OverrideRootScale" null (`self.Damage`) (`self.DamageRadius`) (`self.HitRadialImpulse`) (`self.ProjectileVelocity`) null))

(fn `UserConstructionScript`)